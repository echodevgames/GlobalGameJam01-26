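; Actor that runs a splash screen, then opens the next level by name.
; On BeginPlay it adds the splash widget to the viewport, plays the team splash sound and starts a timer for the configured duration.
; When the timer ends it loads the level; the SkipSplash input clears the timer and, only if the sound component is still valid, stops the sound and advances immediately.
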(event `InputAction|SkipSplash`
  (params (Key :type "Key Structure"))
  (bind _splashsoundcomponent (`self.SplashSoundComponent`))
  (:`Pressed`
    (`KismetSystemLibrary.K2_ClearAndInvalidateTimerHandle` (`self.SplashTimerHandle`))
    (`/Engine/EditorBlueprintResources/StandardMacros.IsValid` _splashsoundcomponent
      (:`Is Valid`
        (`AudioComponent.Stop` _splashsoundcomponent)
        (`self.AdvanceSplash`)))))

(event `self.ReceiveBeginPlay`
  (bind _returnvalue (`|CreateWidget` (`GameplayStatics.GetObjectClass` (`self.SplashWidget`)) (`GameplayStatics.GetPlayerController` 0)))
  (`UserWidget.AddToViewport` _returnvalue 0)
  (bind _returnvalue_2 (`GameplayStatics.SpawnSound2D` "/Game/_Audio/SFX/_TeamSplash._TeamSplash" 1.0 1.0 0.0 null))
  (set `self.SplashSoundComponent` _returnvalue_2)
  (bind _returnvalue_3 (`KismetSystemLibrary.K2_SetTimerDelegate` (delegate `AdvanceSplash`) (`self.Duration`)))
  (set `self.SplashTimerHandle` _returnvalue_3))

(event `AdvanceSplash`
  (`GameplayStatics.OpenLevel` (`self.NextLevelName`)))

(fn `UserConstructionScript`)