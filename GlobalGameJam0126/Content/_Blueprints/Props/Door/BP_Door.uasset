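; Interactable door actor that swings open or shut, but only responds while the player's pickup count equals three.
; On interact it finds BP_Player, checks PickupNum, then calls OpenDoor or CloseDoor based on IsOpen, whose meaning is inverted (true means closed).
; Each plays a sound and runs one timeline forward or in reverse to drive the door's yaw, with a leftover debug print on update.
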(event `OpenDoor`
  ; Door Open/DoorClose
  (set `self.isOpen` false)
  (`GameplayStatics.PlaySoundAtLocation` "/Engine/VREditor/Sounds/UI/Dockable_Window_Open.Dockable_Window_Open" (`self.K2_GetActorLocation`) (struct) 1.0 1.0 0.0 null null null null)
  (bind (_direction _zrot) (`Timeline|OpenDoorTimeLine` :!label _label)
    (:`Update`
      (`SceneComponent.K2_SetRelativeRotation` (`self.Door`) (`KismetMathLibrary.MakeRotator` 0.0 0.0 _zrot) false false)
      (`KismetSystemLibrary.PrintText` "Hello"))))

(event `CloseDoor`
  ; Door Open/DoorClose
  (set `self.isOpen` true)
  (`GameplayStatics.PlaySoundAtLocation` "/Engine/VREditor/Sounds/UI/Dockable_Window_Close.Dockable_Window_Close" (`self.K2_GetActorLocation`) (struct) 1.0 1.0 0.0 null null null null)
  (goto _label :!via `Reverse`))

(event `/Game/_Blueprints/Interface/BPI_Interactable.Oninteract`
  (params (Interactor :type "Actor Object Reference"))
  ; interact
  (bind _returnvalue (`GameplayStatics.GetActorOfClass` "/Game/_Blueprints/Player/BP_Player.BP_Player_C"))
  (if (== (`/Game/_Blueprints/Player/BP_Player.PickupNum` _returnvalue) 3)
    (if (`self.isOpen`)
      (`self.OpenDoor`)
      (else
        (`self.CloseDoor`)))))

(fn `UserConstructionScript`)