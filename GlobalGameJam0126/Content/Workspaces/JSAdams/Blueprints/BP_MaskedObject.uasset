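; BP_MaskedObject is an actor whose mesh shows only in certain states reported by BP_StateManager.
; On BeginPlay it adds its tag, hides the mesh and binds to the manager's state-change notification.
; Each change runs ApplyMaskState, which sets visibility and IsVisible by checking the new state against VisableInStates.
; Interact reports that visibility, with empty output and IsMask false.
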(event `self.ReceiveBeginPlay`
  ; Adds a tag to the object on spawn
  (`KismetArrayLibrary.Array_Add` (`self.Tags`) (`self.Tag`))
  (`SceneComponent.SetVisibility` (`self.Mesh`) false false)
  (bind _returnvalue (`GameplayStatics.GetActorOfClass` "/Game/Workspaces/JSAdams/Blueprints/BP_StateManager.BP_StateManager_C"))
  (add `/Game/Workspaces/JSAdams/Blueprints/BP_StateManager.OnStateChanged` _returnvalue (delegate `OnStateChanged_Bound`)))

(event `OnStateChanged_Bound`
  (params (NewState :type "/Game/_Core/Enums/E_GameModeState Enum" :default "NewEnumerator0"))
  (`self.ApplyMaskState` NewState))

(fn `ApplyMaskState`
  (params (NewState :type "/Game/_Core/Enums/E_GameModeState Enum" :default "NewEnumerator0"))
  (bind _returnvalue (`KismetArrayLibrary.Array_Contains` (`self.VisableInStates`) NewState))
  (`SceneComponent.SetVisibility` (`self.Mesh`) _returnvalue false)
  (set `self.IsVisible` _returnvalue))

(fn `Interact`
  (returns (Output :type Text) (IsMask :type Boolean) (IsVisible :type Boolean))
  (return "" false (`self.IsVisible`)))

(fn `UserConstructionScript`)