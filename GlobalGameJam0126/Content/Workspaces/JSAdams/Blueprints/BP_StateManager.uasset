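; State manager actor that switches the game between Neutral, Reality, Nightmare and Microscopic states, each with its own post-process look.
; ApplyState switches on CurrentState, overwrites the PostProcess settings with a per-state vector, then broadcasts OnStateChanged with that state.
; ApplyPostProcessOffset separately writes a fixed post-process setting without broadcasting.
; The event graph and construction script are empty, so nothing here calls either function.
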(event `self.ReceiveBeginPlay`)

(fn `ApplyPostProcessOffset`
  (set `PostProcessComponent.Settings` (make `PostProcessSettings` :`ColorOffset` (`KismetMathLibrary.MakeVector4` 0.0 0.0 0.0 1.0)) (`self.PostProcess`)))

(fn `ApplyState`
  (switch `/Game/_Core/Enums/E_GameModeState` (`self.CurrentState`)
    (:`NewEnumerator0`
      (set `PostProcessComponent.Settings` (make `PostProcessSettings` :`ColorOffset` (`KismetMathLibrary.MakeVector4` 0.0)) (`self.PostProcess`))
      (`self.OnStateChanged` "NewEnumerator0"))
    (:`NewEnumerator1`
      (set `PostProcessComponent.Settings` (make `PostProcessSettings` :`ColorOffset` (`KismetMathLibrary.MakeVector4` 0.0 0.0 0.0 0.2)) (`self.PostProcess`))
      (`self.OnStateChanged` "NewEnumerator1"))
    (:`NewEnumerator2`
      (set `PostProcessComponent.Settings` (make `PostProcessSettings` :`ColorOffset` (`KismetMathLibrary.MakeVector4` 0.0 0.0 0.0 0.2)) (`self.PostProcess`))
      (`self.OnStateChanged` "NewEnumerator2"))
    (:`NewEnumerator3`
      (set `PostProcessComponent.Settings` (make `PostProcessSettings` :`ColorOffset` (`KismetMathLibrary.MakeVector4` 0.0 0.0 0.0 0.2)) (`self.PostProcess`))
      (`self.OnStateChanged` "NewEnumerator3"))))

(fn `UserConstructionScript`)