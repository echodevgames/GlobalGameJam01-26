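; BP_Trap_GA is a collapsing trap that a player triggers by overlapping its Box.
; It plays a rockfall warning sound, then after a delay plays a cracking impact and hides the StaticMesh with its collision disabled.
; After a second delay the mesh reappears with collision restored.
; The sequence runs on timed Delay nodes in the overlap event and only responds to BP_Player.
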(event `self.Box.OnComponentBeginOverlap`
  (params (OverlappedComponent :type "PrimitiveComponent Object Reference") (OtherActor :type "Actor Object Reference") (OtherComp :type "PrimitiveComponent Object Reference") (OtherBodyIndex :type Integer) (bFromSweep :type Boolean) (SweepResult :type "HitResult Structure (by ref)"))
  (bind _staticmesh (`self.StaticMesh`))
  (bind _staticmesh_2 (`self.StaticMesh`))
  (bind _returnvalue (`SceneComponent.K2_GetComponentLocation` (`self.StaticMesh`)))
  (cast `/Game/_Blueprints/Player/BP_Player` OtherActor)
  (`GameplayStatics.PlaySoundAtLocation` "/Game/_Audio/SFX/In_Game/RockfallRocksFallsDirtSlidesDebris_LJ12A.RockfallRocksFallsDirtSlidesDebris_LJ12A" _returnvalue (struct) 1.0 1.0 0.0 null null null null)
  (`KismetSystemLibrary.Delay` 3.0)
  (`GameplayStatics.PlaySoundAtLocation` "/Game/_Audio/SFX/In_Game/RockCreatureFootstepsHeavyCrackingImpacts_xJmuv_13.RockCreatureFootstepsHeavyCrackingImpacts_xJmuv_13" _returnvalue (struct) 1.0 1.0 0.0 null null null null)
  (`SceneComponent.SetVisibility` _staticmesh_2 false false)
  (`PrimitiveComponent.SetCollisionEnabled` _staticmesh_2 "NoCollision")
  (`KismetSystemLibrary.Delay` 2.0)
  (`SceneComponent.SetVisibility` _staticmesh true false)
  (`PrimitiveComponent.SetCollisionEnabled` _staticmesh "QueryAndPhysics"))

(fn `UserConstructionScript`)